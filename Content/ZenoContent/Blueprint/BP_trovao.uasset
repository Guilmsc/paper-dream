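; One-shot trigger actor that fakes a thunder ("trovao") lightning flash when the player enters its box.
; On overlap by a Player-tagged actor, it turns on every SpotLight tagged Trovao and plays a 2D sound inside that loop, once per light.
; After a 0.2-second delay it finds the tagged lights again, hides them and destroys itself from within that second loop.
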(event OnComponentBeginOverlap(Box)
  (params (OverlappedComponent :type Primitive%20Component%20Object%20Reference) (OtherActor :type Actor%20Object%20Reference) (OtherComp :type Primitive%20Component%20Object%20Reference) (OtherBodyIndex :type Integer) (bFromSweep :type Boolean) (SweepResult :type Hit%20Result%20Structure%20%28by%20ref%29))
  (if (Actor|ActorHasTag OtherActor "Player")
    (bind _outactors (Actor|GetAllActorsOfClass "/Script/Engine.SpotLight"))
    (for _array_element _outactors
      (if (Actor|ActorHasTag _array_element "Trovao")
        (Rendering|SetVisibility (Variables|/Script/Engine.SpotLight|GetSpotLightComponent _array_element) true false)
        (Audio|PlaySound2D "/Engine/EditorSounds/GamePreview/EjectFromPlayer.EjectFromPlayer" 1.0 1.0 0.0 0 0)
        (Utilities|FlowControl|Delay 0.2)
        (bind _outactors_2 (Actor|GetAllActorsOfClasswithTag "/Script/Engine.SpotLight" "Trovao"))
        (for _array_element_2 _outactors_2
          (Rendering|SetVisibility (Variables|/Script/Engine.SpotLight|GetSpotLightComponent _array_element_2) false false)
          (Actor|DestroyActor))))))

(event EventBeginPlay)

(event Collision|EventActorBeginOverlap
  (params (OtherActor :type Actor%20Object%20Reference)))

(event EventTick
  (params (DeltaSeconds :type Float%20%28single-precision%29)))

(fn ConstructionScript)