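; Interactable door Blueprint that swings on its yaw through a three-state cycle: Closed, Partially Open and Open.
; InteractDoor starts the motion and sets a timer, lasting DoorSoundTime, that advances the state.
; Once IsInteracting is set, never cleared here, Tick eases the Door toward the current state's target with FInterpTo.
; Each state targets the following pose: ajar, DoorOpenAngle, or nearly shut, with DoorOpenSide scaling the opening angles.
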(event Custom|HandleRotation
  (params (Rotation :type Float%20%28double-precision%29))
  ;[0.07812 0.07812 0.07812] HandleRotation
  (Transformation|SetRelativeRotation (Variables|Default|GetDoor) (Math|Rotator|MakeRotator 0.0 0.0 (Math|Interpolation|FInterpTo (.Yaw (Math|Rotator|BreakRotator (Variables|/Script/Engine.SceneComponent|GetRelativeRotation (Variables|Default|GetDoor)))) Rotation (Utilities|Time|GetWorldDeltaSeconds) (Variables|Default|GetInterp%20Speed))) false false))

(event Custom|HandleDoor
  ;[0.05208 0.05208 0.05208] HandleDoor
  (switch Utilities|FlowControl|Switch|SwitchonE_DoorStates (Variables|Default|GetdoorStates)
    (:NewEnumerator0
      (CallFunction|HandleRotation (* 15.0 (Variables|Default|GetdoorOpenSide))))
    (:NewEnumerator1
      (CallFunction|HandleRotation (* (Variables|Default|GetdoorOpenAngle) (Variables|Default|GetdoorOpenSide))))
    (:NewEnumerator2
      (CallFunction|HandleRotation 1.0))))

(event Custom|CustomEvent
  ;[0.06771 0.06771 0.06771] Door Interaction
  (Variables|Default|SetisInteracting true)
  (switch Utilities|FlowControl|Switch|SwitchonE_DoorStates (Variables|Default|GetdoorStates)
    (:NewEnumerator0
      (Variables|Default|SetdoorStates "NewEnumerator1"))
    (:NewEnumerator1
      (Variables|Default|SetdoorStates "NewEnumerator2"))
    (:NewEnumerator2
      (Variables|Default|SetdoorStates "NewEnumerator0"))))

(event EventInteractDoor
  (params (charRef :type BP%20Third%20Person%20Character%20Object%20Reference))
  ;[0.06771 0.06771 0.06771] Door Interaction
  (Variables|Default|Setchar%20Ref charRef)
  (Variables|Default|SetisInteracting true)
  (Utilities|Time|SetTimerbyEvent (delegate Custom|CustomEvent) (Variables|Default|GetdoorSoundTime)))

(event EventTick
  (params (DeltaSeconds :type Float%20%28single-precision%29))
  ;[0.06771 0.06771 0.06771] Door Interaction
  (if (Variables|Default|GetisInteracting)
    (CallFunction|HandleDoor)))

(fn ConstructionScript)